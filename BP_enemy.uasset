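; BP_enemy is a Goomba-style enemy that reacts to overlaps on its Goomba component in a two-step sequence.
; The first step adds score and destroys the enemy, but only if the overlapping actor casts to both BP_Player and BP_Projectile.
; The second step subtracts health from player pawn 0, if it is a BP_Player, and destroys the enemy, without checking what overlapped.
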(event `self.Goomba.OnComponentBeginOverlap`
  (params (OverlappedComponent :type "PrimitiveComponent Object Reference") (OtherActor :type "Actor Object Reference") (OtherComp :type "PrimitiveComponent Object Reference") (OtherBodyIndex :type Integer) (bFromSweep :type Boolean) (SweepResult :type "HitResult Structure (by ref)"))
  (`|ExecutionSequence`
    (:`then_0`
      (bind _asbp_player (cast `/Game/InfiniteMatrix/Blueprints/BP_Player` OtherActor))
      (cast `/Game/InfiniteMatrix/Blueprints/BP_Projectile` OtherActor)
      (set `/Game/InfiniteMatrix/Blueprints/BP_Player.Score` (+ (`/Game/InfiniteMatrix/Blueprints/BP_Player.Score` _asbp_player) 200) _asbp_player)
      (`self.K2_DestroyActor`))
    (:`then_1`
      (bind _asbp_player_2 (cast `/Game/InfiniteMatrix/Blueprints/BP_Player` (`GameplayStatics.GetPlayerPawn` 0)))
      (set `/Game/InfiniteMatrix/Blueprints/BP_Player.Health` (`KismetMathLibrary.Conv_IntToDouble` (- (`/Game/InfiniteMatrix/Blueprints/BP_Player.Health` _asbp_player_2) 10)) _asbp_player_2)
      (`self.K2_DestroyActor`))))

(fn `UserConstructionScript`)